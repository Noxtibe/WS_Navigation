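; BPC_SoldierToHeal is an interactable wounded soldier that the player heals while holding something.
; Trigger overlap toggles the mesh's custom-depth outline and a prompt widget, which turns toward the camera every tick.
; Interact calls Heal, which decrements the game mode's remaining-soldier count if IsHolding is true.
; It then adds a new counter widget to the viewport, activates the Healed component and destroys the actor after a delay.
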(event OnComponentBeginOverlap(TriggerArea)
  (params (OverlappedComponent :type Primitive%20Component%20Object%20Reference) (OtherActor :type Actor%20Object%20Reference) (OtherComp :type Primitive%20Component%20Object%20Reference) (OtherBodyIndex :type Integer) (bFromSweep :type Boolean) (SweepResult :type Hit%20Result%20Structure%20%28by%20ref%29))
  ;[1 1 1] Show Outline + Interaction Widget
  (bind _asbp_third_person_character (Utilities|Casting|CastToBP_ThirdPersonCharacter OtherActor))
  (Rendering|SetVisibility (Variables|Default|GetWidget) true false)
  (Rendering|SetRenderCustomDepth (Variables|Character|GetMesh) true))

(event OnComponentEndOverlap(TriggerArea)
  (params (OverlappedComponent :type Primitive%20Component%20Object%20Reference) (OtherActor :type Actor%20Object%20Reference) (OtherComp :type Primitive%20Component%20Object%20Reference) (OtherBodyIndex :type Integer))
  ;[1 1 1] Show Outline + Interaction Widget
  (Utilities|Casting|CastToBP_ThirdPersonCharacter OtherActor)
  (Rendering|SetVisibility (Variables|Default|GetWidget) false false)
  (Rendering|SetRenderCustomDepth (Variables|Character|GetMesh) false))

(event Custom|Heal
  ;[1 1 1] Heal Soldiers and decrease count
  (if (Variables|/Game/Blueprints/Player/BP_ThirdPersonCharacter.BP_ThirdPersonCharacter_C|GetIs%20Holding (stale OnComponentBeginOverlap(TriggerArea) _asbp_third_person_character))
    (bind _asbp_third_person_game_mode (Utilities|Casting|CastToBP_ThirdPersonGameMode (Game|GetGameMode)))
    (bind _result (Math|Integer|DecrementInt (Variables|/Game/Blueprints/Player/BP_ThirdPersonGameMode.BP_ThirdPersonGameMode_C|GetSoldier%20To%20Heal%20Left _asbp_third_person_game_mode))
      (:%20%20
        (Variables|/Game/Blueprints/Player/BP_ThirdPersonGameMode.BP_ThirdPersonGameMode_C|SetSoldier%20To%20Heal%20Left _asbp_third_person_game_mode _result)
        (bind _returnvalue (UserInterface|CreateWidget "/Game/Blueprints/UI/WBP_SoldierToHealLeft.WBP_SoldierToHealLeft_C"))
        (UserInterface|Viewport|AddtoViewport _returnvalue 0)
        (Components|Activation|Activate (Variables|Default|GetHealed) false)
        (Utilities|FlowControl|Delay 1.0)
        (Actor|DestroyActor)))))

(event EventTick
  (params (DeltaSeconds :type Float%20%28single-precision%29))
  ;[1 1 1] Widget follow camera realtime
  (Transformation|SetWorldRotation (Variables|Default|GetWidget) (Math|Rotator|FindLookatRotation (Transformation|GetWorldLocation (Variables|Default|GetWidget)) (Transformation|GetWorldLocation (Variables|/Script/Engine.Actor|GetRootComponent (Game|GetPlayerCameraManager 0)))) false false))

(fn ConstructionScript)

(fn Interact
  (params (Interactor :type Character%20Object%20Reference))
  (CallFunction|Heal)
  (return false))