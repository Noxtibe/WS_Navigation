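; BP_CameraInterior is a trigger actor that changes the third-person camera distance when the player enters or leaves an area, evidently an interior.
; Begin overlap on TriggerCamera plays the InteriorCamera timeline, whose track drives the ThirdPersonCharacter's CameraBoom TargetArmLength.
; End overlap plays a separate BackToExteriorCamera timeline that drives the same arm length for the exterior view.
; Both timelines restart from the beginning on each overlap.
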(event OnComponentBeginOverlap(TriggerCamera)
  (params (OverlappedComponent :type Primitive%20Component%20Object%20Reference) (OtherActor :type Actor%20Object%20Reference) (OtherComp :type Primitive%20Component%20Object%20Reference) (OtherBodyIndex :type Integer) (bFromSweep :type Boolean) (SweepResult :type Hit%20Result%20Structure%20%28by%20ref%29))
  (bind _asbp_third_person_character (Utilities|Casting|CastToBP_ThirdPersonCharacter OtherActor))
  (bind _camera_track (Timeline|Interior%20Camera PlayFromStart)
    (:Update
      (Utilities|IsValid _asbp_third_person_character
        (:Is%20Valid
          (Variables|/Script/Engine.SpringArmComponent|SetTargetArmLength (Variables|/Game/Blueprints/Player/BP_ThirdPersonCharacter.BP_ThirdPersonCharacter_C|GetCameraBoom _asbp_third_person_character) _camera_track))))))

(event OnComponentEndOverlap(TriggerCamera)
  (params (OverlappedComponent :type Primitive%20Component%20Object%20Reference) (OtherActor :type Actor%20Object%20Reference) (OtherComp :type Primitive%20Component%20Object%20Reference) (OtherBodyIndex :type Integer))
  (bind _asbp_third_person_character (Utilities|Casting|CastToBP_ThirdPersonCharacter OtherActor))
  (bind _camera_track (Timeline|Back%20to%20Exterior%20Camera PlayFromStart)
    (:Update
      (Utilities|IsValid _asbp_third_person_character
        (:Is%20Valid
          (Variables|/Script/Engine.SpringArmComponent|SetTargetArmLength (Variables|/Game/Blueprints/Player/BP_ThirdPersonCharacter.BP_ThirdPersonCharacter_C|GetCameraBoom _asbp_third_person_character) _camera_track))))))

(event EventBeginPlay)

(fn ConstructionScript)