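; Interactable door actor that toggles open and closed, swinging its Scene component by yaw along a timeline each time Interact is called.
; An overlap box detects the third-person character, showing a prompt widget, enabling custom depth on the door for highlighting, and running timelines that change the character's camera boom length.
; Leaving the box reverses these effects with a separate dezoom timeline.
; The widget turns every tick to face the player camera.
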(event OnComponentBeginOverlap(Box)
  (params (OverlappedComponent :type Primitive%20Component%20Object%20Reference) (OtherActor :type Actor%20Object%20Reference) (OtherComp :type Primitive%20Component%20Object%20Reference) (OtherBodyIndex :type Integer) (bFromSweep :type Boolean) (SweepResult :type Hit%20Result%20Structure%20%28by%20ref%29))
  (bind _asbp_third_person_character (Utilities|Casting|CastToBP_ThirdPersonCharacter OtherActor))
  (Rendering|SetVisibility (Variables|Default|GetWidget) true false)
  (Rendering|SetRenderCustomDepth (Variables|Default|GetDoor) true)
  (bind _camera_track (Timeline|Camera%20Zoom PlayFromStart)
    (:Update
      (Utilities|IsValid _asbp_third_person_character
        (:Is%20Valid
          (Variables|/Script/Engine.SpringArmComponent|SetTargetArmLength (Variables|/Game/Blueprints/Player/BP_ThirdPersonCharacter.BP_ThirdPersonCharacter_C|GetCameraBoom _asbp_third_person_character) _camera_track))))))

(event OnComponentEndOverlap(Box)
  (params (OverlappedComponent :type Primitive%20Component%20Object%20Reference) (OtherActor :type Actor%20Object%20Reference) (OtherComp :type Primitive%20Component%20Object%20Reference) (OtherBodyIndex :type Integer))
  (bind _asbp_third_person_character (Utilities|Casting|CastToBP_ThirdPersonCharacter OtherActor))
  (Rendering|SetVisibility (Variables|Default|GetWidget) false false)
  (Rendering|SetRenderCustomDepth (Variables|Default|GetDoor) false)
  (bind _camera_track (Timeline|Camera%20Dezoom PlayFromStart)
    (:Update
      (Utilities|IsValid _asbp_third_person_character
        (:Is%20Valid
          (Variables|/Script/Engine.SpringArmComponent|SetTargetArmLength (Variables|/Game/Blueprints/Player/BP_ThirdPersonCharacter.BP_ThirdPersonCharacter_C|GetCameraBoom _asbp_third_person_character) _camera_track))))))

(event Custom|Opening%20Door
  ;[1 1 1] Anim Door
  (Utilities|FlowControl|FlipFlop
    (:A
      (bind _door_track (Timeline|OpeningDoor Play)
        (:Update
          (Transformation|SetRelativeRotation (Variables|Default|GetScene) (Math|Rotator|MakeRotator 0.0 0.0 (Math|Float|Lerp 0.0 -9e+01 _door_track)) false false))))
    (:B
      (Timeline|OpeningDoor Reverse))))

(event EventTick
  (params (DeltaSeconds :type Float%20%28single-precision%29))
  ;[1 1 1] Show widget
  (Transformation|SetWorldRotation (Variables|Default|GetWidget) (Math|Rotator|FindLookatRotation (Transformation|GetWorldLocation (Variables|Default|GetWidget)) (Transformation|GetWorldLocation (Variables|/Script/Engine.Actor|GetRootComponent (Game|GetPlayerCameraManager 0)))) false false))

(fn ConstructionScript)

(fn Interact
  (params (Interactor :type Character%20Object%20Reference))
  (CallFunction|OpeningDoor)
  (return true))